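; Procedurally generated room that builds itself on BeginPlay, sized and populated from the GameInstance's difficulty and seeded random stream.
; Tiles instanced floor and wall meshes, scattering zombies, spitters and mines while counting enemies left to kill.
; Unless it is the last room, three exit doors get non-repeating random gene types or a rare special type.
; A loaded game skips spawning enemies and mines and fires the level-complete dispatcher.
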(event `self.ReceiveBeginPlay`
  (bind _gameinstance (`self.GameInstance`))
  (`self.InitializeVariables`)
  (`self.BuildRoom`)
  (if (`/Game/TopDown/BP_LabRatInstance.IsLoaded` _gameinstance)
    (`/Game/TopDown/BP_LabRatInstance.LevelCompleteDispatcher` _gameinstance)
    (set `/Game/TopDown/BP_LabRatInstance.IsLoaded` false _gameinstance)))

(fn `BuildFloorAndStuff`
  (bind (_returnvalue_x _returnvalue_y) (`KismetMathLibrary.BreakVector` (`self.K2_GetActorLocation`)))
  (bind _xtilescount (`self.XTilesCount`))
  (bind _gameinstance (`self.GameInstance`))
  (bind _random (`/Game/TopDown/BP_LabRatInstance.Random` (`self.GameInstance`)))
  ;[0 0 0] Build the floor of the room
  (for _index (range _xtilescount)
    (for _index_2 (range (`self.YTilesCount`))
      (bind _returnvalue (* _index (`self.XTileSize`)))
      (bind _returnvalue_2 (* _index_2 (`self.YTileSize`)))
      (`InstancedStaticMeshComponent.AddInstance` (`self.Floor`) (`KismetMathLibrary.MakeTransform` (`KismetMathLibrary.MakeVector` _returnvalue _returnvalue_2)) false)
      ;[0 0 0] Spawn enemies
      (if (and (not (`/Game/TopDown/BP_LabRatInstance.IsLoaded` (`self.GameInstance`))) (and (> _index 1) (< _index (- _xtilescount 2))))
        (if (`KismetMathLibrary.RandomBoolWithWeightFromStream` _random (+ 0.4 (* (`self.Difficulty`) 0.02)))
          (if (`KismetMathLibrary.RandomBoolWithWeightFromStream` _random 0.75)
            (bind _returnvalue_3 (`KismetMathLibrary.MakeVector` (+ (+ _returnvalue _returnvalue_x) 200.0) (+ (+ _returnvalue_2 _returnvalue_y) 200.0) 100.0))
            (`|SpawnActorFromClass` "/Game/Enemies/Zombie/BP_Zombie.BP_Zombie_C" (`KismetMathLibrary.MakeTransform` _returnvalue_3) "Undefined" "MultiplyWithRoot" null null)
            (else
              (`|SpawnActorFromClass` "/Game/Enemies/Spitter/BP_Spitter.BP_Spitter_C" (`KismetMathLibrary.MakeTransform` _returnvalue_3) "Undefined" "MultiplyWithRoot" null null)))
          (set `/Game/TopDown/BP_LabRatInstance.EnemiesLeftToKill` (+ (`/Game/TopDown/BP_LabRatInstance.EnemiesLeftToKill` _gameinstance) 1) _gameinstance)
          (elif (`KismetMathLibrary.RandomBoolWithWeightFromStream` (`/Game/TopDown/BP_LabRatInstance.Random` (`self.GameInstance`)) (+ 0.2 (* (`self.Difficulty`) 0.02)))
            (`|SpawnActorFromClass` "/Game/LevelGeneration/BP_Mine.BP_Mine_C" (`KismetMathLibrary.MakeTransform` (- _returnvalue_3 (0.0 0.0 100.0)) (struct) (1.3 1.3 1.3)) "Undefined" "MultiplyWithRoot" null null)))))))

(fn `BuildRoom`
  (`self.BuildFloorAndStuff`)
  (`self.BuildWallsAndDoors`))

(fn `BuildWallsAndDoors`
  (locals (RandomIndex :type Integer))
  (bind (_returnvalue_x _returnvalue_y) (`KismetMathLibrary.BreakVector` (`self.K2_GetActorLocation`)))
  (bind _ytilescount (`self.YTilesCount`))
  (bind _genetypes (`self.GeneTypes`))
  (bind _returnvalue (/ _ytilescount 2))
  (bind _random (`/Game/TopDown/BP_LabRatInstance.Random` (`self.GameInstance`)))
  ;[0 0 0] Build the X-parallel walls
  (for _index (range (`self.XTilesCount`))
    (bind _returnvalue_2 (* _index (`self.XTileSize`)))
    (`InstancedStaticMeshComponent.AddInstance` (`self.Wall`) (`KismetMathLibrary.MakeTransform` (`KismetMathLibrary.MakeVector` _returnvalue_2)) false)
    (`InstancedStaticMeshComponent.AddInstance` (`self.Wall`) (`KismetMathLibrary.MakeTransform` (`KismetMathLibrary.MakeVector` _returnvalue_2 (* (`self.YTilesCount`) (`self.YTileSize`)))) false))
  ;[0 0 0] Build the Y-parallel walls, the doors
  (for _index_2 (range _ytilescount)
    (bind _returnvalue_3 (* _index_2 (`self.YTileSize`)))
    (`InstancedStaticMeshComponent.AddInstance` (`self.Wall`) (`KismetMathLibrary.MakeTransform` (`KismetMathLibrary.MakeVector` 0.0 _returnvalue_3) (struct :`Yaw` 90.0)) false)
    (if (and (or (or (== _index_2 (- _returnvalue 2)) (== _index_2 _returnvalue)) (== _index_2 (+ _returnvalue 2))) (not (`self.IsTheLastRoom`)))
      (if (`KismetMathLibrary.RandomBoolWithWeightFromStream` _random 0.05)
        (bind _returnvalue_4 (`KismetMathLibrary.MakeVector` (* (`self.XTilesCount`) (`self.XTileSize`)) _returnvalue_3))
        (bind _returnvalue_5 (+ (.x _returnvalue_4) _returnvalue_x))
        (bind _returnvalue_6 (+ (+ (.y _returnvalue_4) (`self.YTileSize`)) _returnvalue_y))
        (`|SpawnActorFromClass` "/Game/LevelGeneration/BP_Door.BP_Door_C" (`KismetMathLibrary.MakeTransform` (`KismetMathLibrary.MakeVector` _returnvalue_5 _returnvalue_6) (struct :`Yaw` -90.0)) "Undefined" "MultiplyWithRoot" null "NewEnumerator5" null)
        (else
          (bind _output_get (set `local.RandomIndex` (`KismetMathLibrary.RandomIntegerInRangeFromStream` _random 0 (- (`KismetArrayLibrary.Array_Length` _genetypes) 1))))
          (`|SpawnActorFromClass` "/Game/LevelGeneration/BP_Door.BP_Door_C" (`KismetMathLibrary.MakeTransform` (`KismetMathLibrary.MakeVector` _returnvalue_5 _returnvalue_6) (struct :`Yaw` -90.0)) "Undefined" "MultiplyWithRoot" null (`|GetArrayItem` _genetypes _output_get) null)
          (`KismetArrayLibrary.Array_Remove` _genetypes _output_get)))
      (else
        (`InstancedStaticMeshComponent.AddInstance` (`self.Wall`) (`KismetMathLibrary.MakeTransform` _returnvalue_4 (struct :`Yaw` 90.0)) false)))))

(fn `InitializeVariables`
  (bind _difficulty (`self.Difficulty`))
  (bind _returnvalue (/ _difficulty 2))
  (bind _returnvalue_2 (/ _difficulty 3))
  ;[0 0 0] Initialize variables based on game instance
  (bind _asbp_lab_rat_instance (cast `/Game/TopDown/BP_LabRatInstance` (`GameplayStatics.GetGameInstance`)))
  (set `self.GameInstance` _asbp_lab_rat_instance)
  (set `self.Difficulty` (`/Game/TopDown/BP_LabRatInstance.Difficulty` _asbp_lab_rat_instance))
  (bind _random (`/Game/TopDown/BP_LabRatInstance.Random` _asbp_lab_rat_instance))
  (set `self.XTilesCount` (`KismetMathLibrary.RandomIntegerInRangeFromStream` _random (+ _returnvalue_2 7) (+ _returnvalue 7)))
  (set `self.YTilesCount` (`KismetMathLibrary.RandomIntegerInRangeFromStream` _random (+ _returnvalue_2 7) (+ _returnvalue 7)))
  (if (== (`/Game/TopDown/BP_LabRatInstance.CurrentRoom` _asbp_lab_rat_instance) (`/Game/TopDown/BP_LabRatInstance.TotalRooms` _asbp_lab_rat_instance))
    (set `self.IsTheLastRoom` true)))

(fn `UserConstructionScript`
  ;[1 1 1] Connect for in-editor testing
)