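; Game instance for LabRat that holds level-generation and combat state: current room, random stream and enemies left to kill.
; On Init it resets the room index and enemy count to zero and seeds the random stream.
; KillEnemy decrements the enemy count and fires the victory dispatcher when it reaches exactly zero.
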(event `self.ReceiveInit`
  (`self.Initialize`))

(event `Event KillEnemy`
  (bind _output_get (set `self.EnemiesLeftToKill` (- (`self.EnemiesLeftToKill`) 1)))
  (if (== _output_get 0)
    (`self.VictoryDispatcher`)))

(fn `Initialize`
  ;[1 1 1] Initialize game instance
  (set `self.CurrentRoom` 0)
  (`KismetMathLibrary.SeedRandomStream` (`self.Random`))
  (set `self.EnemiesLeftToKill` 0))