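; BP_Mine is a proximity mine hazard that explodes when the top-down player character overlaps it.
; A timeline started on BeginPlay drives the point light's intensity to make it blink.
; On overlap with BP_TopDownCharacter it applies fixed damage, spawns an explosion particle effect and destroys itself.
; Its IsDead function always returns false.
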(event `self.ReceiveBeginPlay`
  (bind (_direction _lightintensitytrack) (`Timeline|LightBlinkTimeLine`)
    (:`Update`
      (`LightComponent.SetIntensity` (`self.PointLight`) _lightintensitytrack))))

(event `self.ReceiveActorBeginOverlap`
  (params (OtherActor :type "Actor Object Reference"))
  (bind _asbp_top_down_character (cast `/Game/TopDown/Blueprints/Character/BP_TopDownCharacter` OtherActor))
  (`GameplayStatics.ApplyDamage` _asbp_top_down_character 30.0 null self)
  (`GameplayStatics.SpawnEmitterAtLocation` "/Game/StarterContent/Particles/P_Explosion.P_Explosion" (`self.K2_GetActorLocation`) (struct) (1.3 1.3 1.3))
  (`self.K2_DestroyActor`))

(fn `IsDead`
  (returns (IsDead :type Boolean))
  (return false))

(fn `UserConstructionScript`)