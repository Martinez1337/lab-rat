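; BP_Door is a level exit that loads the generated map for the next room once the current level is complete.
; The game instance's level-complete dispatcher makes it usable, and an optional red material is applied on BeginPlay.
; Player overlap binds the interact dispatcher to the door, and leaving clears all bindings on that dispatcher.
; Using the door increments difficulty and current room in the game instance before opening the map.
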(event `self.ReceiveBeginPlay`
  ;[1 1 1] Initialize
  (if (`self.IsRed`)
    (`PrimitiveComponent.SetMaterial` (`self.Door`) 1 "/Game/StarterContent/Materials/M_RedDoor.M_RedDoor"))
  (bind _asbp_lab_rat_instance (cast `/Game/TopDown/BP_LabRatInstance` (`GameplayStatics.GetGameInstance`)))
  (bind _output_get (set `self.GameInstance` _asbp_lab_rat_instance))
  (add `/Game/TopDown/BP_LabRatInstance.LevelCompleteDispatcher` _output_get (delegate `Make Door Useable`)))

(event `Make Door Useable`
  ;[1 1 1] Initialize
  (set `self.IsUseable` true))

(event `self.ReceiveActorBeginOverlap`
  (params (OtherActor :type "Actor Object Reference"))
  (cast `/Game/TopDown/Blueprints/Character/BP_TopDownCharacter` OtherActor)
  (add `/Game/TopDown/BP_LabRatInstance.InteractDispatcher` (`self.GameInstance`) (delegate `OpenNextLevel`)))

(event `OpenNextLevel`
  (bind _gameinstance (`self.GameInstance`))
  (if (`self.IsUseable`)
    (set `/Game/TopDown/BP_LabRatInstance.Difficulty` (+ (`/Game/TopDown/BP_LabRatInstance.Difficulty` _gameinstance) 1) _gameinstance)
    (set `/Game/TopDown/BP_LabRatInstance.CurrentRoom` (+ (`/Game/TopDown/BP_LabRatInstance.CurrentRoom` _gameinstance) 1) _gameinstance)
    (`GameplayStatics.OpenLevelBySoftObjectPtr` "/Game/TopDown/Maps/GeneratedMap.GeneratedMap")))

(event `self.ReceiveActorEndOverlap`
  (params (OtherActor :type "Actor Object Reference"))
  (cast `/Game/TopDown/Blueprints/Character/BP_TopDownCharacter` OtherActor)
  (clear `/Game/TopDown/BP_LabRatInstance.InteractDispatcher` (`self.GameInstance`)))

(fn `UserConstructionScript`)