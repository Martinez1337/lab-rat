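; BP_SpitShooter is an enemy Spitter's projectile launcher that fires spit balls from a pre-spawned pool.
; BeginPlay spawns half-scale BP_SpitBall actors in a loop over Size and stores them in SpitBalls.
; Shoot moves the ball at CurrentIndex to the shooter's location and launches it along the forward vector.
; CurrentIndex then advances and resets near Size, so balls are recycled instead of spawned per shot.
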(event `self.ReceiveBeginPlay`
  ;[1 1 1] Spawn spit balls
  (for _ (range (+ (`self.Size`) 1))
    (bind _returnvalue (`|SpawnActorFromClass` "/Game/Enemies/Spitter/BP_SpitBall.BP_SpitBall_C" (`KismetMathLibrary.MakeTransform` (0.0 0.0 0.0) (struct) (0.5 0.5 0.5)) "Undefined" "MultiplyWithRoot" null null))
    (`KismetArrayLibrary.Array_Add` (`self.SpitBalls`) _returnvalue)))

(event `Shoot`
  (bind _output (`|GetArrayItem` (`self.SpitBalls`) (`self.CurrentIndex`)))
  (bind _returnvalue (+ (`self.CurrentIndex`) 1))
  ;[1 1 1] Shoot spit balls
  (`self.K2_SetActorLocation` _output (`self.K2_GetActorLocation`) false false)
  (`/Game/Enemies/Spitter/BP_SpitBall.Shoot` _output (`self.GetActorForwardVector`))
  (set `self.CurrentIndex` _returnvalue)
  (if (== _returnvalue (`self.Size`))
    (set `self.CurrentIndex` 0)))

(fn `UserConstructionScript`)