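; Spit ball projectile for the Spitter enemy that deals fixed damage to the top-down player character on overlap.
; Shoot launches it along the given direction at the movement component's initial speed, enabling overlaps and showing the sphere.
; Hitting the player or any actor not implementing BI_Enemy stops and hides it instead of destroying it, so it can be shot again.
; It passes through BI_Enemy actors, and its IsDead always returns false.
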(event `self.ReceiveActorBeginOverlap`
  (params (OtherActor :type "Actor Object Reference"))
  (bind _asbp_top_down_character (cast `/Game/TopDown/Blueprints/Character/BP_TopDownCharacter` OtherActor)
    (:`then`
      (`GameplayStatics.ApplyDamage` _asbp_top_down_character 25.0 null self)
      (`ProjectileMovementComponent.SetVelocityInLocalSpace` (`self.ProjectileMovement`) (0.0 0.0 0.0) :!label _label)
      (set `PrimitiveComponent.bGenerateOverlapEvents` false (`self.Collision`))
      (`SceneComponent.SetVisibility` (`self.Sphere`) false false))
    (:`CastFailed`
      (if (not (`KismetSystemLibrary.DoesImplementInterface` OtherActor "/Game/Enemies/BI_Enemy.BI_Enemy_C"))
        (goto _label)))))

(event `Shoot`
  (params (Forward :type "Vector Structure"))
  (bind _projectilemovement (`self.ProjectileMovement`))
  (`ProjectileMovementComponent.SetVelocityInLocalSpace` _projectilemovement (* Forward (`ProjectileMovementComponent.InitialSpeed` _projectilemovement)))
  (set `PrimitiveComponent.bGenerateOverlapEvents` true (`self.Collision`))
  (`SceneComponent.SetVisibility` (`self.Sphere`) true false))

(fn `IsDead`
  (returns (IsDead :type Boolean))
  (return false))

(fn `UserConstructionScript`)