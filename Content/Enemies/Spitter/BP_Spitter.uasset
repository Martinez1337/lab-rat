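; BP_Spitter is an enemy with health, a radial melee-range attack and a ragdoll death.
; Only damage caused by BP_TopDownCharacter reduces its health, with each hit spawning a short-lived explosion effect.
; At zero health it clears its animation class, enables mesh physics, disables movement and capsule collision, then reports the kill to BP_LabRatInstance.
; The Attack event deals full damage within a small radius around itself.
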(event `self.ReceiveBeginPlay`
  (set `self.CurrentHealth` (`self.MaxHealth`)))

(event `self.ReceiveAnyDamage`
  (params (Damage :type "Float (single-precision)") (DamageType :type "DamageType Object Reference") (InstigatedBy :type "Controller Object Reference") (DamageCauser :type "Actor Object Reference"))
  (if (not (`self.IsDeadBool`))
    (cast `/Game/TopDown/Blueprints/BP_TopDownCharacter` DamageCauser)
    (set `self.CurrentHealth` (`KismetMathLibrary.FClamp` (- (`self.CurrentHealth`) Damage) 0.0 (`self.MaxHealth`)))
    (bind _returnvalue (`GameplayStatics.SpawnEmitterAtLocation` "/Game/StarterContent/Particles/P_Explosion.P_Explosion" (`self.K2_GetActorLocation`)))
    (`KismetSystemLibrary.K2_SetTimerDelegate` (delegate `Event DestroyEmitter`) 0.2)
    (if (== (`self.CurrentHealth`) 0.0)
      (`self.Event Death`))))

(event `Event DestroyEmitter`
  (`ActorComponent.K2_DestroyComponent` (stale `self.ReceiveAnyDamage` _returnvalue)))

(event `Event Death`
  (bind _mesh (`self.Mesh`))
  (bind _charactermovement (`self.CharacterMovement`))
  (set `self.IsDeadBool` true)
  (`SkeletalMeshComponent.SetAnimInstanceClass` _mesh null)
  (`PrimitiveComponent.SetSimulatePhysics` _mesh true)
  (`MovementComponent.StopMovementImmediately` _charactermovement)
  (`CharacterMovementComponent.DisableMovement` _charactermovement)
  (`PrimitiveComponent.SetCollisionEnabled` (`self.CapsuleComponent`) "NoCollision")
  (bind _asbp_lab_rat_instance (cast `/Game/LevelGeneration/BP_LabRatInstance` (`GameplayStatics.GetGameInstance`)))
  (`/Game/LevelGeneration/BP_LabRatInstance.Event KillEnemy` _asbp_lab_rat_instance))

(event `/Game/Enemies/BI_Enemy.Attack`
  (`GameplayStatics.ApplyRadialDamage` :`BaseDamage` 25.0 :`Origin` (`self.K2_GetActorLocation`) :`DamageRadius` 150.0 :`DamageCauser` self :`InstigatedByController` null :`bDoFullDamage` true))

(fn `IsDead`
  (returns (IsDead :type Boolean))
  (return (`self.IsDeadBool`)))

(fn `UserConstructionScript`)