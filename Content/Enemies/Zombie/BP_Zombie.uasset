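; Zombie enemy character with health that takes damage only from BP_TopDownCharacter and deals radial damage around itself when it attacks.
; Each valid hit lowers clamped health and spawns scaled-up blood particles; the timer meant to destroy the emitter is never run.
; At zero health it ragdolls, disables movement and capsule collision, and reports the kill to BP_LabRatInstance, with IsDead exposing the state.
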(event `self.ReceiveBeginPlay`
  ;[1 1 1] Set full health
  (set `self.CurrentHealth` (`self.MaxHealth`)))

(event `self.ReceiveAnyDamage`
  (params (Damage :type "Float (single-precision)") (DamageType :type "DamageType Object Reference") (InstigatedBy :type "Controller Object Reference") (DamageCauser :type "Actor Object Reference"))
  ;[1 1 1] Get hit
  (if (not (`self.IsDeadBool`))
    (cast `/Game/TopDown/Blueprints/BP_TopDownCharacter` DamageCauser)
    (set `self.CurrentHealth` (`KismetMathLibrary.FClamp` (- (`self.CurrentHealth`) Damage) 0.0 (`self.MaxHealth`)))
    (bind _returnvalue (`GameplayStatics.SpawnEmitterAtLocation` "/Game/StarterContent/Particles/P_Blood.P_Blood" (`self.K2_GetActorLocation`) (struct) (4.0 4.0 4.0)))
    (if (== (`self.CurrentHealth`) 0.0)
      (`self.Event Death`))))

(event `Event DestroyEmitter`
  ;[1 1 1] Get hit
  (`ActorComponent.K2_DestroyComponent` (stale `self.ReceiveAnyDamage` _returnvalue)))

(event `Event Death`
  (bind _mesh (`self.Mesh`))
  (bind _charactermovement (`self.CharacterMovement`))
  ;[1 1 1] Die
  (set `self.IsDeadBool` true)
  (`SkeletalMeshComponent.SetAnimInstanceClass` _mesh null)
  (`PrimitiveComponent.SetSimulatePhysics` _mesh true)
  (`MovementComponent.StopMovementImmediately` _charactermovement)
  (`CharacterMovementComponent.DisableMovement` _charactermovement)
  (`PrimitiveComponent.SetCollisionEnabled` (`self.CapsuleComponent`) "NoCollision")
  (bind _asbp_lab_rat_instance (cast `/Game/LevelGeneration/BP_LabRatInstance` (`GameplayStatics.GetGameInstance`)))
  (`/Game/LevelGeneration/BP_LabRatInstance.Event KillEnemy` _asbp_lab_rat_instance))

(event `/Game/Enemies/BI_Enemy.Attack`
  ;[1 1 1] Attack
  (`GameplayStatics.ApplyRadialDamage` :`BaseDamage` 25.0 :`Origin` (`self.K2_GetActorLocation`) :`DamageRadius` 200.0 :`DamageCauser` self :`InstigatedByController` null :`bDoFullDamage` true))

(fn `IsDead`
  (returns (IsDead :type Boolean))
  (return (`self.IsDeadBool`)))

(fn `UserConstructionScript`)