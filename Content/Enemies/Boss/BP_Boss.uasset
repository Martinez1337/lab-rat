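; BP_Boss is a boss enemy character whose max health scales with the player's win count.
; Damage updates its HP bar, spawns blood and notifies the player, while attacks are delegated to a child-actor BP_BossShooter.
; Piercing Claws upgrades add bleed stacks, ticked by a looping timer using BP_BleedingDamage so bleed hits add no further stacks.
; Death enables mesh ragdoll, disables movement and capsule collision, removes the bar and reports the kill.
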(event `self.ReceiveBeginPlay`
  ;[1 1 1] Initialize
  (bind _asbp_boss_shooter (cast `/Game/Enemies/Boss/BP_BossShooter` (`ChildActorComponent.ChildActor` (`self.BP_BossShooter`))))
  (set `self.Shooter` _asbp_boss_shooter)
  (bind _asbp_lab_rat_instance (cast `/Game/TopDown/BP_LabRatInstance` (`GameplayStatics.GetGameInstance`)))
  (bind _output_get (set `self.GameInstance` _asbp_lab_rat_instance))
  (bind _output_get_2 (set `self.MaxHealth` (+ (`self.MaxHealth`) (* (`/Game/TopDown/BP_LabRatInstance.WinsCount` _output_get) 100))))
  (set `self.CurrentHealth` _output_get_2)
  (bind _returnvalue (`KismetSystemLibrary.K2_SetTimerDelegate` (delegate `Event Bleed`) 1.0 true))
  (set `self.BleedingTimer` _returnvalue)
  (bind _aswbp_hpbar (cast `/Game/UI/HUD/WBP_HPBar` (`WidgetComponent.GetWidget` (`self.HP Bar`))))
  (`Widget.SetRenderScale` _aswbp_hpbar (3.0 1.2)))

(event `Event Bleed`
  ;[1 1 1] Initialize
  (if (> (`self.Bleeding`) 0)
    (`GameplayStatics.ApplyDamage` self (`KismetMathLibrary.Conv_IntToDouble` (`self.Bleeding`)) null (`GameplayStatics.GetPlayerCharacter` 0) "/Game/Enemies/BP_BleedingDamage.BP_BleedingDamage_C")
    (set `self.Bleeding` (- (`self.Bleeding`) 1))))

(event `self.ReceiveAnyDamage`
  (params (Damage :type "Float (single-precision)") (DamageType :type "DamageType Object Reference") (InstigatedBy :type "Controller Object Reference") (DamageCauser :type "Actor Object Reference"))
  (bind _gameinstance (`self.GameInstance`))
  ;[1 1 1] Get hit
  (if (not (`self.IsDeadBool`))
    (bind _asbp_top_down_character (cast `/Game/TopDown/Blueprints/Character/BP_TopDownCharacter` DamageCauser))
    (`/Game/TopDown/Blueprints/Character/BP_TopDownCharacter.Event Enemy Hit` _asbp_top_down_character (`KismetMathLibrary.FClamp` Damage 0.0 (`self.CurrentHealth`)))
    (bind _output_get (set `self.CurrentHealth` (`KismetMathLibrary.FClamp` (- (`self.CurrentHealth`) Damage) 0.0 (`self.MaxHealth`))))
    (bind _aswbp_hpbar (cast `/Game/UI/HUD/WBP_HPBar` (`WidgetComponent.GetWidget` (`self.HP Bar`))))
    (`/Game/UI/HUD/WBP_HPBar.UpdateHealthUI` _aswbp_hpbar _output_get (`self.MaxHealth`))
    (`GameplayStatics.SpawnEmitterAtLocation` "/Game/StarterContent/Particles/P_Blood.P_Blood" (`self.K2_GetActorLocation`) (struct) (8.0 8.0 8.0))
    (if (<= (`self.CurrentHealth`) 0.0)
      (`self.Event Death`)
      (else
        (cast `/Game/Enemies/BP_BleedingDamage` DamageType
          (:`CastFailed`
            (if (`/Game/TopDown/BP_LabRatInstance.HasPiercingClaws` _gameinstance)
              (if (`/Game/TopDown/BP_LabRatInstance.HasPiercingClawsII` _gameinstance)
                (set `self.Bleeding` (+ (`self.Bleeding`) 4))
                (else
                  (set `self.Bleeding` (+ (`self.Bleeding`) 2)))))))))))

(event `Event Death`
  (bind _mesh (`self.Mesh`))
  (bind _charactermovement (`self.CharacterMovement`))
  ;[1 1 1] Die
  (set `self.IsDeadBool` true)
  (`SkeletalMeshComponent.SetAnimInstanceClass` _mesh null)
  (`PrimitiveComponent.SetSimulatePhysics` _mesh true)
  (`MovementComponent.StopMovementImmediately` _charactermovement)
  (`CharacterMovementComponent.DisableMovement` _charactermovement)
  (`PrimitiveComponent.SetCollisionEnabled` (`self.CapsuleComponent`) "NoCollision")
  (`ActorComponent.K2_DestroyComponent` (`self.HP Bar`))
  (`/Game/TopDown/BP_LabRatInstance.Event KillEnemy` (`self.GameInstance`))
  (`KismetSystemLibrary.K2_PauseTimerHandle` (`self.BleedingTimer`)))

(event `/Game/Enemies/BI_Enemy.Attack`
  (`/Game/Enemies/Boss/BP_BossShooter.Shoot` (`self.Shooter`)))

(fn `IsDead`
  (returns (IsDead :type Boolean))
  (return (`self.IsDeadBool`)))

(fn `UserConstructionScript`)